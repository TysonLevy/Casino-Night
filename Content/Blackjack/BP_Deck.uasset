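; BP_Deck runs a blackjack round, acting as both deck and dealer.
; A Tick-driven GameState machine spawns and shuffles BP_Playing_Card actors, deals two hands, runs player and dealer turns, then prints the outcome.
; Clickable Hit, Stay and Deal buttons act only in their matching state, with Deal clearing the table for a new round.
; ScoreHand totals a hand, demoting aces from 11 to 1 to avoid busting.
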(event OnClicked(Stay_Button)
  (params (TouchedComponent :type Primitive%20Component%20Object%20Reference) (ButtonPressed :type Key%20Structure :default "None"))
  (Math|Integer|CompareInt (Variables|Default|GetGameState) 1
    (:==
      (Variables|Default|SetGameState 2))))

(event OnClicked(Hit_Button)
  (params (TouchedComponent :type Primitive%20Component%20Object%20Reference) (ButtonPressed :type Key%20Structure :default "None"))
  (bind _playerhand (Variables|Default|GetPlayerHand))
  (bind _returnvalue (Utilities|Array|Length _playerhand))
  (Math|Integer|CompareInt (Variables|Default|GetGameState) 1
    (:==
      (Utilities|Array|Insert _playerhand (Utilities|Array|Get(acopy) (Variables|Default|GetCards) (Variables|Default|GetCard%20Count)) _returnvalue)
      (Transformation|SetActorTransform (Utilities|Array|Get(acopy) (Variables|Default|GetCards) (Variables|Default|GetCard%20Count)) (Math|Transform|MakeTransform (Math|Vector|MakeVector -2e+01 (Math|Conversions|ToFloat(Integer) (+ (* _returnvalue 10) -80)) 1.9e+02) "180.000000,0.000000,0.000000" "0.100000,0.100000,1.000000"))
      (bind _result (Math|Integer|IncrementInt (Variables|Default|GetCard%20Count))
        (:%20%20
          (Variables|Default|SetCard%20Count _result))))))

(event OnClicked(Deal_Button)
  (params (TouchedComponent :type Primitive%20Component%20Object%20Reference) (ButtonPressed :type Key%20Structure :default "None"))
  (Math|Integer|CompareInt (Variables|Default|GetGameState) 4
    (:==
      (for _array_element (Variables|Default|GetCards)
        (Actor|DestroyActor _array_element))
      (Variables|Default|SetCard%20Count 0)
      (Utilities|Array|Clear (Variables|Default|GetCards))
      (Utilities|Array|Clear (Variables|Default|GetPlayerHand))
      (Utilities|Array|Clear (Variables|Default|GetDealerHand))
      (Variables|Default|SetPlayerBust false)
      (Variables|Default|SetDealerBust false)
      (Variables|Default|SetGameState 0))))

(event EventBeginPlay)

(event Collision|EventActorBeginOverlap
  (params (OtherActor :type Actor%20Object%20Reference)))

(event EventTick
  (params (DeltaSeconds :type Float%20%28single-precision%29))
  (bind _dealerhand (Variables|Default|GetDealerHand))
  (bind _cards (Variables|Default|GetCards))
  (bind _dealerhand_2 (Variables|Default|GetDealerHand))
  (bind _sm_playingcard (Variables|Default|GetSM_PlayingCard))
  (bind _cards_2 (Variables|Default|GetCards))
  (bind _playerhand (Variables|Default|GetPlayerHand))
  (bind _returnvalue (Utilities|Array|Length _dealerhand_2))
  (bind _returnvalue_2 (Transformation|GetRelativeTransform _sm_playingcard))
  (bind _output (Utilities|Array|Get(acopy) _cards 3))
  (bind _output_2 (Utilities|Array|Get(acopy) _cards_2))
  (bind _output_3 (Utilities|Array|Get(acopy) _cards_2 1))
  (bind _output_4 (Utilities|Array|Get(acopy) _cards_2 2))
  (bind _output_5 (Utilities|Array|Get(acopy) _cards_2 3))
  (bind (_location _rotation) (Math|Transform|BreakTransform _returnvalue_2))
  (bind _returnvalue_3 (Transformation|GetActorTransform _output))
  (bind (_location_2 _rotation_2 _scale) (Math|Transform|BreakTransform _returnvalue_3))
  (switch int (Variables|Default|GetGameState)
    (:0
      ;[1 1 1] Shuffle Deck
      (bind _enumvalue (|ForEachE_CardRanks)
        (:LoopBody
          (bind _enumvalue_2 (|ForEachE_CardSuits)
            (:LoopBody
              (bind _returnvalue_4 (Game|SpawnActorfromClass "/Game/HG_Playing_Cards/Blueprints/BP_Playing_Card.BP_Playing_Card_C" (Math|Transform|MakeTransform _location _rotation "0.100000,0.100000,1.000000") "AdjustIfPossibleButAlwaysSpawn" "MultiplyWithRoot" 0 0))
              (Default|SetCardValue _returnvalue_4 "NewEnumerator0" _enumvalue_2 _enumvalue "NewEnumerator1")
              (Utilities|Array|Insert (Variables|Default|GetCards) _returnvalue_4 (Variables|Default|GetCard%20Count))
              (bind _result (Math|Integer|IncrementInt (Variables|Default|GetCard%20Count))
                (:%20%20
                  (Variables|Default|SetCard%20Count _result))))))
        (:then
          (Utilities|Array|Shuffle (Variables|Default|GetCards))
          (Utilities|Array|Insert _playerhand _output_2)
          (Utilities|Array|Insert _playerhand _output_3 1)
          (Utilities|Array|Insert _dealerhand _output_4)
          (Utilities|Array|Insert _dealerhand _output_5 1)
          (Transformation|SetActorTransform _output_2 (Math|Transform|MakeTransform "-20.000000,-70.000000,190.000000" "180.000000,0.000000,0.000000" "0.100000,0.100000,1.000000"))
          (Transformation|SetActorTransform _output_3 (Math|Transform|MakeTransform "-20.000000,-60.000000,190.000000" "180.000000,0.000000,0.000000" "0.100000,0.100000,1.000000"))
          (Transformation|SetActorTransform _output_4 (Math|Transform|MakeTransform "60.000000,-70.000000,190.000000" "180.000000,0.000000,0.000000" "0.100000,0.100000,1.000000"))
          (Transformation|SetActorTransform _output_5 (Math|Transform|MakeTransform "60.000000,-60.000000,190.000000" "0.000000,0.000000,0.000000" "0.100000,0.100000,1.000000"))
          (Variables|Default|SetCard%20Count 4)
          (Variables|Default|SetGameState 1))))
    (:1
      (bind _score (CallFunction|ScoreHand (Variables|Default|GetPlayerHand)))
      (Math|Integer|CompareInt _score 20
        (:>
          (Variables|Default|SetGameState 2))))
    (:2
      (Transformation|SetActorTransform _output (Math|Transform|MakeTransform _location_2 "180.000000,0.000000,0.000000" _scale))
      (bind _score_2 (CallFunction|ScoreHand (Variables|Default|GetDealerHand) :!label _label))
      (Math|Integer|CompareInt _score_2 16
        (:>
          _)
        (:==
          _)
        (:<
          (Utilities|Array|Insert _dealerhand_2 (Utilities|Array|Get(acopy) (Variables|Default|GetCards) (Variables|Default|GetCard%20Count)) _returnvalue)
          (Transformation|SetActorTransform (Utilities|Array|Get(acopy) (Variables|Default|GetCards) (Variables|Default|GetCard%20Count)) (Math|Transform|MakeTransform (Math|Vector|MakeVector 6e+01 (Math|Conversions|ToFloat(Integer) (+ (* _returnvalue 10) -80)) 1.9e+02) "180.000000,0.000000,0.000000" "0.100000,0.100000,1.000000"))
          (bind _result_2 (Math|Integer|IncrementInt (Variables|Default|GetCard%20Count))
            (:%20%20
              (Variables|Default|SetCard%20Count _result_2)
              (goto _label)))))
      (Variables|Default|SetGameState 3))
    (:3
      (bind _score_3 (CallFunction|ScoreHand (Variables|Default|GetPlayerHand)))
      (Math|Integer|CompareInt _score_3 21
        (:>
          (Variables|Default|SetPlayerBust true))
        (:==
          _)
        (:<
          _))
      (Math|Integer|CompareInt _score_2 21
        (:>
          (Variables|Default|SetDealerBust true))
        (:==
          _)
        (:<
          _))
      (if (or (Variables|Default|GetPlayerBust) (Variables|Default|GetDealerBust))
        (if (and (Variables|Default|GetPlayerBust) (Variables|Default|GetDealerBust))
          (Variables|Default|SetOutcome "Tie!" :!label _label_2)
          (elif (Variables|Default|GetDealerBust)
            (Variables|Default|SetOutcome "Win!" :!label _label_3)
            (else
              (Variables|Default|SetOutcome "Lose!" :!label _label_4))))
        (else
          (Math|Integer|CompareInt _score_3 _score_2
            (:>
              (goto _label_3))
            (:==
              (goto _label_2))
            (:<
              (goto _label_4)))))
      (Development|PrintString (Variables|Default|GetOutcome) true true "(R=0.000000,G=0.660000,B=1.000000,A=1.000000)" 5.0)
      (Variables|Default|SetGameState 4))))

(fn ConstructionScript)

(fn ScoreHand
  (params (Hand :type Array%20of%20BP%20Playing%20Card%20Object%20References))
  (Variables|Default|SetScore 0)
  (Variables|Default|SetAceCount 0)
  (for _array_element Hand
    (bind _value (Default|ScoreCard _array_element))
    (Math|Integer|CompareInt _value 11
      (:>
        _)
      (:==
        (Math|Integer|IncrementInt (Variables|Default|GetAceCount)
          (:%20%20
            _)))
      (:<
        _))
    (Variables|Default|SetScore (+ _value (Variables|Default|GetScore))))
  (Math|Integer|CompareInt (Variables|Default|GetScore) 21 :!label _label
    (:>
      (Math|Integer|CompareInt (Variables|Default|GetAceCount)
        (:>
          (Math|Integer|DecrementInt (Variables|Default|GetAceCount)
            (:%20%20
              (Variables|Default|SetScore (+ (Variables|Default|GetScore) -10))
              (goto _label))))
        (:==
          _)
        (:<
          _)))
    (:==
      _)
    (:<
      _))
  (return (Variables|Default|GetScore)))